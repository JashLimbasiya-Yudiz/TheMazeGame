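; Maze wall actor that opens as the player approaches and closes again once the player leaves.
; When the player character begins overlapping Box2, the Wall is hidden with collision disabled, and two pillars become visible and solid.
; When the player stops overlapping a separate volume, Box, the swap reverses, restoring the solid Wall and removing both pillars.
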(event `self.Box2.OnComponentBeginOverlap`
  (params (OverlappedComponent :type "PrimitiveComponent Object Reference") (OtherActor :type "Actor Object Reference") (OtherComp :type "PrimitiveComponent Object Reference") (OtherBodyIndex :type Integer) (bFromSweep :type Boolean) (SweepResult :type "HitResult Structure (by ref)"))
  (bind _pillar1 (`self.Pillar1`))
  (bind _wall (`self.Wall`))
  (if (== OtherActor (`GameplayStatics.GetPlayerCharacter` 0))
    (`SceneComponent.SetVisibility` _wall false false)
    (`PrimitiveComponent.SetCollisionEnabled` _wall "NoCollision")
    (`SceneComponent.SetVisibility` _pillar1 true false)
    (`SceneComponent.SetVisibility` (`self.Pillar2`) true false)
    (`PrimitiveComponent.SetCollisionEnabled` _pillar1 "QueryAndPhysics")
    (`PrimitiveComponent.SetCollisionEnabled` (`self.Pillar2`) "QueryAndPhysics")))

(event `self.Box.OnComponentEndOverlap`
  (params (OverlappedComponent :type "PrimitiveComponent Object Reference") (OtherActor :type "Actor Object Reference") (OtherComp :type "PrimitiveComponent Object Reference") (OtherBodyIndex :type Integer))
  (bind _pillar1 (`self.Pillar1`))
  (if (== OtherActor (`GameplayStatics.GetPlayerCharacter` 0))
    (`SceneComponent.SetVisibility` (`self.Wall`) true false)
    (`PrimitiveComponent.SetCollisionEnabled` (`self.Wall`) "QueryAndPhysics")
    (`SceneComponent.SetVisibility` _pillar1 false false)
    (`SceneComponent.SetVisibility` (`self.Pillar2`) false false)
    (`PrimitiveComponent.SetCollisionEnabled` _pillar1 "NoCollision")
    (`PrimitiveComponent.SetCollisionEnabled` (`self.Pillar2`) "NoCollision")))

(fn `UserConstructionScript`)