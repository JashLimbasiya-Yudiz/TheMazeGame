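; KeyPlatform is a maze pickup pedestal holding a Skull Key that the player collects with the Interact input.
; Its trigger volume enables input and shows a HUD prompt while the player overlaps, then disables input and clears it on exit.
; Pickup destroys the key component, adds its index and component reference to the PlayerCharacter, refreshes the HUD through MazeGameMode and plays a sound.
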(event `InputAction|Interect`
  (params (Key :type "Key Structure"))
  (:`Pressed`
    (`/Engine/EditorBlueprintResources/StandardMacros.IsValid` (`self.Key`)
      (:`Is Valid`
        (`ActorComponent.K2_DestroyComponent` (`self.Key`))
        (bind _asplayer_character (cast `/Game/MyMazeGame/Blueprints/PlayerCharacter` (`GameplayStatics.GetPlayerCharacter` 0)))
        (`KismetArrayLibrary.Array_Add` (`/Game/MyMazeGame/Blueprints/PlayerCharacter.Keys` _asplayer_character) (`self.KeyIndex`))
        (`KismetArrayLibrary.Array_Add` (`/Game/MyMazeGame/Blueprints/PlayerCharacter.KeyMeshes` _asplayer_character) (`self.Key`))
        (bind _asmaze_game_mode (cast `/Game/MyMazeGame/Blueprints/MazeGameMode` (`GameplayStatics.GetGameMode`)))
        (bind _headsupdisplay (`/Game/MyMazeGame/Blueprints/MazeGameMode.HeadsUpDisplay` _asmaze_game_mode))
        (`/Game/MyMazeGame/UI/WidgetBlueprintd/HeadsUpDisplay.UpdateKeys` _headsupdisplay)
        (set `/Game/MyMazeGame/UI/WidgetBlueprintd/HeadsUpDisplay.Message` "" _headsupdisplay)
        (`/Game/MyMazeGame/UI/WidgetBlueprintd/HeadsUpDisplay.UpdateMessage` _headsupdisplay)
        (`GameplayStatics.PlaySoundAtLocation` "/Game/MyMazeGame/Sounds/PickupSkull_SFX.PickupSkull_SFX" (`self.K2_GetActorLocation` (`GameplayStatics.GetPlayerCharacter` 0)) (struct) 1.0 1.0 0.0 null null null)))))

(event `self.TriggerVolume.OnComponentBeginOverlap`
  (params (OverlappedComponent :type "PrimitiveComponent Object Reference") (OtherActor :type "Actor Object Reference") (OtherComp :type "PrimitiveComponent Object Reference") (OtherBodyIndex :type Integer) (bFromSweep :type Boolean) (SweepResult :type "HitResult Structure (by ref)"))
  (if (== OtherActor (`GameplayStatics.GetPlayerCharacter` 0))
    (`self.EnableInput` (`GameplayStatics.GetPlayerController` 0))
    (`/Engine/EditorBlueprintResources/StandardMacros.IsValid` (`self.Key`)
      (:`Is Valid`
        (bind _asmaze_game_mode (cast `/Game/MyMazeGame/Blueprints/MazeGameMode` (`GameplayStatics.GetGameMode`)))
        (bind _headsupdisplay (`/Game/MyMazeGame/Blueprints/MazeGameMode.HeadsUpDisplay` _asmaze_game_mode))
        (set `/Game/MyMazeGame/UI/WidgetBlueprintd/HeadsUpDisplay.Message` "Press \"E\" to pick up the Skull Key" _headsupdisplay)
        (`/Game/MyMazeGame/UI/WidgetBlueprintd/HeadsUpDisplay.UpdateMessage` _headsupdisplay)))))

(event `self.TriggerVolume.OnComponentEndOverlap`
  (params (OverlappedComponent :type "PrimitiveComponent Object Reference") (OtherActor :type "Actor Object Reference") (OtherComp :type "PrimitiveComponent Object Reference") (OtherBodyIndex :type Integer))
  (if (== OtherActor (`GameplayStatics.GetPlayerCharacter` 0))
    (`self.DisableInput` (`GameplayStatics.GetPlayerController` 0))
    (bind _asmaze_game_mode (cast `/Game/MyMazeGame/Blueprints/MazeGameMode` (`GameplayStatics.GetGameMode`)))
    (bind _headsupdisplay (`/Game/MyMazeGame/Blueprints/MazeGameMode.HeadsUpDisplay` _asmaze_game_mode))
    (set `/Game/MyMazeGame/UI/WidgetBlueprintd/HeadsUpDisplay.Message` "" _headsupdisplay)
    (`/Game/MyMazeGame/UI/WidgetBlueprintd/HeadsUpDisplay.UpdateMessage` _headsupdisplay)))

(fn `UserConstructionScript`)