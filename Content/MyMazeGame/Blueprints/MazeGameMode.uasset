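; Game mode for the maze game that owns the HUD widget and handles the win and lose endings.
; BeginPlay creates the HUD, and ShowInfoMessage briefly reveals its info text before hiding it again.
; Win and Lose disable player input, fade the camera to white or red, and remove the HUD.
; After a short delay, each shows its end-screen widget and switches to UI-only input with a visible cursor.
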(event `ShowInfoMessage`
  (bind _infomessage (`/Game/MyMazeGame/UI/WidgetBlueprintd/HeadsUpDisplay.InfoMessage` (`self.HeadsUpDisplay`)))
  (`Widget.SetVisibility` _infomessage "Visible")
  (`KismetSystemLibrary.Delay` 2.0)
  (`Widget.SetVisibility` _infomessage "Hidden"))

(event `self.ReceiveBeginPlay`
  (bind _returnvalue (`|CreateWidget` "/Game/MyMazeGame/UI/WidgetBlueprintd/HeadsUpDisplay.HeadsUpDisplay_C"))
  (bind _output_get (set `self.HeadsUpDisplay` _returnvalue))
  (`UserWidget.AddToViewport` _output_get 0))

(event `Lose`
  (bind _returnvalue (`GameplayStatics.GetPlayerController` 0))
  (`self.DisableInput` (`GameplayStatics.GetPlayerCharacter` 0) (`GameplayStatics.GetPlayerController` 0))
  (`PlayerCameraManager.StartCameraFade` (`GameplayStatics.GetPlayerCameraManager` 0) 0.0 0.8 2.0 (struct :`R` 0.895833 :`G` 0.058893 :`B` 0.044792 :`A` 1.0) false true)
  (`Widget.RemoveFromParent` (`self.HeadsUpDisplay`))
  (`KismetSystemLibrary.Delay` 2.0)
  (bind _returnvalue_2 (`|CreateWidget` "/Game/MyMazeGame/UI/WidgetBlueprintd/LoseScreen.LoseScreen_C"))
  (`UserWidget.AddToViewport` _returnvalue_2 0)
  (`WidgetBlueprintLibrary.SetInputMode_UIOnlyEx` _returnvalue _returnvalue_2)
  (set `PlayerController.bShowMouseCursor` true _returnvalue))

(event `Win`
  (bind _returnvalue (`GameplayStatics.GetPlayerController` 0))
  (`self.DisableInput` (`GameplayStatics.GetPlayerCharacter` 0) (`GameplayStatics.GetPlayerController` 0))
  (`PlayerCameraManager.StartCameraFade` (`GameplayStatics.GetPlayerCameraManager` 0) 0.0 0.8 2.0 (struct :`R` 1.0 :`G` 1.0 :`B` 1.0 :`A` 1.0) false true)
  (`Widget.RemoveFromParent` (`self.HeadsUpDisplay`))
  (`KismetSystemLibrary.Delay` 2.0)
  (bind _returnvalue_2 (`|CreateWidget` "/Game/MyMazeGame/UI/WidgetBlueprintd/WinScreen.WinScreen_C"))
  (`UserWidget.AddToViewport` _returnvalue_2 0)
  (`WidgetBlueprintLibrary.SetInputMode_UIOnlyEx` _returnvalue _returnvalue_2)
  (set `PlayerController.bShowMouseCursor` true _returnvalue))

(fn `UserConstructionScript`)